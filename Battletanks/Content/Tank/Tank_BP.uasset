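; Tank_BP is a player-controllable tank pawn that aims, fires and drives on two independently throttled tracks.
; On BeginPlay it passes its barrel, turret and track components to setter functions defined outside this graph.
; Aim axes rotate an azimuth gimbal for yaw and a spring arm for pitch, orbiting the camera.
; Throttle axes feed each track separately, and the Fire action calls Fire.
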(event EventBeginPlay
  (Class|Tank|SetBarrelReference (Variables|Default|GetBarrel))
  (Class|Tank|SetTurretReference (Variables|Default|GetTankTurret))
  (Class|Tank|SetTracksReferences (Variables|Default|GetLeft%20Track) (Variables|Default|GetRight%20Track)))

(event Input|ActionEvents|InputActionFire
  (params (Key :type Key%20Structure))
  ;[1 1 1] Fire
  (:Pressed
    (Class|Tank|Fire)))

(event Input|AxisEvents|InputAxisAimAzimuth
  (params (AxisValue :type Float%20%28single-precision%29))
  ;[1 1 1] Camera
  (Transformation|AddLocalRotation (Variables|Default|GetAzimuth%20Gimbal) (Math|Rotator|MakeRotator 0.0 0.0 (* AxisValue 2.0)) false false))

(event Input|AxisEvents|InputAxisLeftAxisThrottle
  (params (AxisValue :type Float%20%28single-precision%29))
  ;[1 1 1] Movement
  (Class|TankTrack|SetThrottle (Variables|Default|GetLeft%20Track) AxisValue))

(event Input|AxisEvents|InputAxisAimEleveation
  (params (AxisValue :type Float%20%28single-precision%29))
  ;[1 1 1] Camera
  (Transformation|AddLocalRotation (Variables|Default|GetSpringArm) (Math|Rotator|MakeRotator 0.0 (* AxisValue 2.0) 0.0) false false))

(event Input|AxisEvents|InputAxisRightAxisThrottle
  (params (AxisValue :type Float%20%28single-precision%29))
  ;[1 1 1] Movement
  (Class|TankTrack|SetThrottle (Variables|Default|GetRight%20Track) AxisValue))

(fn ConstructionScript)